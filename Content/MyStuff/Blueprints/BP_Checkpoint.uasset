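; BP_Checkpoint is a checkpoint actor that saves the player's respawn point and updates the level shown in the UI.
; When its Cube is hit by the first-person character, it writes the TPPoint component's world transform into the game mode's RespawnTransform.
; It then passes its LevelNumber to the UI through the game mode's UIRef.
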(event OnComponentHit(Cube)
  (params (HitComponent :type Primitive%20Component%20Object%20Reference) (OtherActor :type Actor%20Object%20Reference) (OtherComp :type Primitive%20Component%20Object%20Reference) (NormalImpulse :type Vector :default "0, 0, 0") (Hit :type Hit%20Result%20Structure%20%28by%20ref%29))
  (bind _returnvalue (Actor|GetActorOfClass "/Game/FirstPerson/Blueprints/BP_FirstPersonCharacter.BP_FirstPersonCharacter_C"))
  (if (== _returnvalue OtherActor)
    (bind _asbp_first_person_game_mode (Utilities|Casting|CastToBP_FirstPersonGameMode (Game|GetGameMode)))
    (Variables|/Game/FirstPerson/Blueprints/BP_FirstPersonGameMode.BP_FirstPersonGameMode_C|SetRespawn%20Transform _asbp_first_person_game_mode (Transformation|GetWorldTransform (Variables|Default|GetTPPoint)))
    (bind _asbp_first_person_game_mode_2 (Utilities|Casting|CastToBP_FirstPersonGameMode (Game|GetGameMode)))
    (Default|UpdateLevel (Variables|/Game/FirstPerson/Blueprints/BP_FirstPersonGameMode.BP_FirstPersonGameMode_C|GetUIRef _asbp_first_person_game_mode_2) (Variables|Default|GetLevelNumber))))

(fn ConstructionScript)